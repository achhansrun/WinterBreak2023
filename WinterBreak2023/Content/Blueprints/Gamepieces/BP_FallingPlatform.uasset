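; BP_FallingPlatform is a platform that moves toward an end location when BP_Player enters its trigger box and returns when the player leaves.
; The MovePlatform timeline plays or reverses on overlap, scaled by a configurable duration, lerping MainPlatform's relative location from its BeginPlay position to EndLocation.
; The construction script applies mesh, scale and rotation to both MainPlatform and EndPlatformRef, placing the latter at EndLocation to mark the destination.
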(event `self.ReceiveBeginPlay`
  (set `self.start Location` (`SceneComponent.RelativeLocation` (`self.mainPlatform`))))

(event `self.Box.OnComponentBeginOverlap`
  (params (OverlappedComponent :type "PrimitiveComponent Object Reference") (OtherActor :type "Actor Object Reference") (OtherComp :type "PrimitiveComponent Object Reference") (OtherBodyIndex :type Integer) (bFromSweep :type Boolean) (SweepResult :type "HitResult Structure (by ref)"))
  (castclass `/Game/Blueprints/Player/BP_Player` "/Game/Blueprints/Player/BP_Player.BP_Player_C")
  (`TimelineComponent.SetPlayRate` (`self.MovePlatform`) (`KismetMathLibrary.SafeDivide` 1.0 (`self.duration(in sec)`)))
  (bind (_direction _move_track) (`Timeline|MovePlatform` :!label _label)
    (:`Update`
      (`SceneComponent.K2_SetRelativeLocation` (`self.mainPlatform`) (`KismetMathLibrary.VLerp` (`self.start Location`) (`self.end Location`) _move_track) false false))))

(event `self.Box.OnComponentEndOverlap`
  (params (OverlappedComponent :type "PrimitiveComponent Object Reference") (OtherActor :type "Actor Object Reference") (OtherComp :type "PrimitiveComponent Object Reference") (OtherBodyIndex :type Integer))
  (castclass `/Game/Blueprints/Player/BP_Player` "/Game/Blueprints/Player/BP_Player.BP_Player_C")
  (`TimelineComponent.SetPlayRate` (`self.MovePlatform`) (`KismetMathLibrary.SafeDivide` 1.0 (`self.duration(in sec)`)))
  (goto _label :!via `Reverse`))

(fn `UserConstructionScript`
  (bind _mainplatform (`self.mainPlatform`))
  (bind _endplatformref (`self.endPlatformRef`))
  (bind _platformmesh (`self.platformMesh`))
  (`StaticMeshComponent.SetStaticMesh` _mainplatform _platformmesh)
  (`StaticMeshComponent.SetStaticMesh` _endplatformref _platformmesh)
  (`SceneComponent.SetRelativeScale3D` _mainplatform (`self.scale`))
  (`SceneComponent.SetRelativeScale3D` _endplatformref (`self.scale`))
  (`SceneComponent.K2_SetRelativeRotation` _mainplatform (`self.rotation`) false false)
  (`SceneComponent.K2_SetRelativeRotation` _endplatformref (`self.rotation`) false false)
  (`SceneComponent.K2_SetRelativeLocation` _endplatformref (`self.end Location`) false false))