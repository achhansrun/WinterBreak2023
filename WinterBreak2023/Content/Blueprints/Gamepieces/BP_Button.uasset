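; BP_Button is an interactable push-button gamepiece with a placeholder action that prints "Button pressed".
; A box overlap opens a gate only while BP_Player is inside, letting Interact trigger the ButtonAnimation graph.
; That graph plays a sound and uses two timelines to lerp the button in and back out.
; Its output hangs off the return timeline's Update, so the action fires on every update of that stroke.
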(event `self.ReceiveBeginPlay`
  (bind (_returnvalue_location _returnvalue_rotation _returnvalue_scale) (`KismetMathLibrary.BreakTransform` (`SceneComponent.GetRelativeTransform` (`self.Button`))))
  (set `self.Out Position` (`KismetMathLibrary.MakeTransform` _returnvalue_location _returnvalue_rotation _returnvalue_scale))
  (set `self.In Position` (`KismetMathLibrary.MakeTransform` (- _returnvalue_location (0.0 30.0 0.0)) _returnvalue_rotation _returnvalue_scale))
  (`self.EnableInput` (`GameplayStatics.GetPlayerController` 0)))

(event `/Game/Blueprints/Interfaces/interactInterface.interact`
  (params (Player :type "CharacterEvent Structure"))
  ;[1 1 1] Button interaction push button
  (`/Engine/EditorBlueprintResources/StandardMacros.Gate` true :!label _label
    (:`Exit`
      ;[1 1 1] Button Moving animation
      (`GameplayStatics.PlaySoundAtLocation` null (`self.K2_GetActorLocation`) (struct) 1.0 1.0 0.0 null null null null)
      (bind (_direction _newtrack_0) (`Timeline|Button In` :!via `PlayFromStart`)
        (:`Update`
          (`SceneComponent.K2_SetRelativeTransform` (`self.Button`) (`KismetMathLibrary.TLerp` (`self.Out Position`) (`self.In Position`) _newtrack_0) false false))
        (:`Finished`
          (bind (_direction_2 _newtrack_0_2) (`Timeline|Button Out` :!via `ReverseFromEnd`)
            (:`Update`
              (`SceneComponent.K2_SetRelativeTransform` (`self.Button`) (`KismetMathLibrary.TLerp` (`self.Out Position`) (`self.In Position`) _newtrack_0_2) false false)
              ;[1 1 1] Code you want button to execute
              (`KismetSystemLibrary.PrintString` "Button pressed" true true (struct :`G` 0.66 :`B` 1.0 :`A` 1.0) 1.0))))))))

(event `self.Box.OnComponentBeginOverlap`
  (params (OverlappedComponent :type "PrimitiveComponent Object Reference") (OtherActor :type "Actor Object Reference") (OtherComp :type "PrimitiveComponent Object Reference") (OtherBodyIndex :type Integer) (bFromSweep :type Boolean) (SweepResult :type "HitResult Structure (by ref)"))
  ;[1 1 1] Button interaction push button
  (cast `/Game/Blueprints/Player/BP_Player` OtherActor)
  (goto _label :!via `Open`))

(event `self.Box.OnComponentEndOverlap`
  (params (OverlappedComponent :type "PrimitiveComponent Object Reference") (OtherActor :type "Actor Object Reference") (OtherComp :type "PrimitiveComponent Object Reference") (OtherBodyIndex :type Integer))
  ;[1 1 1] Button interaction push button
  (cast `/Game/Blueprints/Player/BP_Player` OtherActor)
  (goto _label :!via `Close`))

(fn `UserConstructionScript`)