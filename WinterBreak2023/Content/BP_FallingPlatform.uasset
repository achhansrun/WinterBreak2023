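; BP_FallingPlatform is a platform actor whose construction script previews a main platform and an end-position reference.
; Both components share the same configurable mesh, scale and rotation, and the reference is placed at the EndLocation relative offset.
; The event graph holds only disabled placeholder events, so this graph contains no falling or movement logic.
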(fn `UserConstructionScript`
  (bind _mainplatform (`self.mainPlatform`))
  (bind _endplatformref (`self.endPlatformRef`))
  (bind _platformmesh (`self.platformMesh`))
  (`StaticMeshComponent.SetStaticMesh` _mainplatform _platformmesh)
  (`StaticMeshComponent.SetStaticMesh` _endplatformref _platformmesh)
  (`SceneComponent.SetRelativeScale3D` _mainplatform (`self.scale`))
  (`SceneComponent.SetRelativeScale3D` _endplatformref (`self.scale`))
  (`SceneComponent.K2_SetRelativeRotation` _mainplatform (`self.rotation`) false false)
  (`SceneComponent.K2_SetRelativeRotation` _endplatformref (`self.rotation`) false false)
  (`SceneComponent.K2_SetRelativeLocation` _endplatformref (`self.end Location`) false false))